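; Sword-wielding NPC character that fights the player in melee and can be assassinated.
; An attack event plays a combo montage, while sword hitbox overlaps damage the player when attack-ready, throttled by a DoOnce and short delay.
; Taking damage lowers and prints health and plays a hit reaction, with no death check.
; An area overlap toggles the player's CanAssassinate flag, and TakeDown plays an ambush montage before ragdolling body and weapon.
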(event `self.ReceiveBeginPlay`
  (`SceneComponent.K2_AttachToComponent` (`self.WeaponMesh`) (`self.Mesh`) "Weapon1_R" "SnapToTarget" "SnapToTarget" "SnapToTarget" true))

(event `/Game/Blueprints/NPC/NPC1/AI/INT_NPCCombat.NPCMeleeAttack`
  ;[1 1 1] Plays the attack animation montage for the NPC
  (`|PlayMontage` (`self.Mesh`) "/Game/Characters/NPC/Animation/NPCSword_Combo_1_Montage.NPCSword_Combo_1_Montage"))

(event `self.ReceiveAnyDamage`
  (params (Damage :type "Float (single-precision)") (DamageType :type "DamageType Object Reference") (InstigatedBy :type "Controller Object Reference") (DamageCauser :type "Actor Object Reference"))
  ;[1 1 1] Take Damage and reset attack if hit
  (bind _output_get (set `self.Health` (- (`self.Health`) Damage)))
  (`KismetSystemLibrary.PrintString` (`KismetStringLibrary.Conv_DoubleToString` _output_get))
  (`self.PlayAnimMontage` "/Game/Characters/PlayerCharacter/Animations/Standing_React_Large_From_Front_Montage.Standing_React_Large_From_Front_Montage"))

(event `self.SwordHitBix.OnComponentBeginOverlap`
  (params (OverlappedComponent :type "PrimitiveComponent Object Reference") (OtherActor :type "Actor Object Reference") (OtherComp :type "PrimitiveComponent Object Reference") (OtherBodyIndex :type Integer) (bFromSweep :type Boolean) (SweepResult :type "HitResult Structure (by ref)"))
  ;[1 1 1] Deal Damage
  (bind _asplayer_character_bare_bp (cast `/Game/Blueprints/PlayerCharacter/PlayerCharacterBare_BP` OtherActor))
  (if (`self.AttackReady_0`)
    (`/Engine/EditorBlueprintResources/StandardMacros.DoOnce` false :!label _label
      (:`Completed`
        (`GameplayStatics.ApplyDamage` _asplayer_character_bare_bp 10.0)
        (`KismetSystemLibrary.Delay` 0.4)
        (goto _label :!via `Reset`)))))

(event `self.AssassinateArea.OnComponentBeginOverlap`
  (params (OverlappedComponent :type "PrimitiveComponent Object Reference") (OtherActor :type "Actor Object Reference") (OtherComp :type "PrimitiveComponent Object Reference") (OtherBodyIndex :type Integer) (bFromSweep :type Boolean) (SweepResult :type "HitResult Structure (by ref)"))
  (bind _asplayer_character_bare_bp (cast `/Game/Blueprints/PlayerCharacter/PlayerCharacterBare_BP` OtherActor))
  (set `/Game/Blueprints/PlayerCharacter/PlayerCharacterBare_BP.CanAssassinate?` true _asplayer_character_bare_bp))

(event `self.AssassinateArea.OnComponentEndOverlap`
  (params (OverlappedComponent :type "PrimitiveComponent Object Reference") (OtherActor :type "Actor Object Reference") (OtherComp :type "PrimitiveComponent Object Reference") (OtherBodyIndex :type Integer))
  (bind _asplayer_character_bare_bp (cast `/Game/Blueprints/PlayerCharacter/PlayerCharacterBare_BP` OtherActor))
  (set `/Game/Blueprints/PlayerCharacter/PlayerCharacterBare_BP.CanAssassinate?` false _asplayer_character_bare_bp))

(event `TakeDown`
  (`CharacterMovementComponent.DisableMovement` (`self.CharacterMovement`))
  (`self.SetActorEnableCollision` false)
  (`self.PlayAnimMontage` "/Game/Characters/NPC/Animation/TwinSword_Attack_Ambushed_Montage.TwinSword_Attack_Ambushed_Montage")
  (`KismetSystemLibrary.Delay` 5.2)
  (`self.Ragdoll`))

(event `Ragdoll`
  (bind _weaponmesh (`self.WeaponMesh`))
  ;[1 1 1] Ragdoll Physics
  (`PrimitiveComponent.SetSimulatePhysics` (`self.Mesh`) true)
  (`CharacterMovementComponent.DisableMovement` (`self.CharacterMovement`))
  (`PrimitiveComponent.SetCollisionProfileName` _weaponmesh "ragdoll" true)
  (`PrimitiveComponent.SetSimulatePhysics` _weaponmesh true))

(fn `UserConstructionScript`)