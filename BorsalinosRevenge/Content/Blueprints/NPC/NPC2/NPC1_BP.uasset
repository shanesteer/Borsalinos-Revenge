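; Melee enemy NPC with a socketed weapon and a health bar widget that shows while the player overlaps its detection sphere.
; Its sword hitbox damages the player through a delayed DoOnce gate, while incoming damage updates the bar and plays a hit reaction.
; Death or stealth assassination ragdolls it, drops a coin and destroys it.
; Stealth eligibility comes from an AI blackboard flag; the dodge event is marked unused.
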(event `self.ReceiveBeginPlay`
  (`SceneComponent.K2_AttachToComponent` (`self.WeaponMesh`) (`self.Mesh`) "Weapon_R1" "SnapToTarget" "SnapToTarget" "SnapToTarget" true)
  (bind _asai_health_bar_wb (cast `/Game/Blueprints/NPC/NPC2/AI/AI_HealthBarWB` (`WidgetComponent.GetUserWidgetObject` (`self.Widget`))))
  (set `self.HealthWidgetREF` _asai_health_bar_wb))

(event `/Game/Blueprints/NPC/NPC2/AI/NPC_AI_INT.Dodge Away`
  (params (`Focused Actor` :type "Actor Object Reference"))
  ;[1 1 1] For dodging away from player character(Unused)
  (if (not (`self.IsPlayingRootMotion`))
    (set `self.Focused Actor` `Focused Actor`)
    (`self.PlayAnimMontage` "/Game/Characters/NPC2/Animation/NPC_Dodge_Montage.NPC_Dodge_Montage")))

(event `/Game/Blueprints/NPC/NPC2/AI/NPC_AI_INT.ExecuteStealth`
  ;[1 1 1] Playing anim Montage for assasination
  (`CharacterMovementComponent.SetMovementMode` (`self.CharacterMovement`) "MOVE_None" 0)
  (set `/Game/Blueprints/NPC/NPC2/AI/AI_HealthBarWB.Health` 0.0 (`self.HealthWidgetREF`))
  (`PrimitiveComponent.SetCollisionResponseToChannel` (`self.CapsuleComponent`) "ECC_Pawn" "ECR_Overlap")
  (`ActorComponent.K2_DestroyComponent` (`self.SwordHitBox`))
  (`self.PlayAnimMontage` "/Game/Characters/NPC2/Animation/TwinSword_Attack_Ambushed_Montage.TwinSword_Attack_Ambushed_Montage")
  (`CharacterMovementComponent.SetMovementMode` (`self.CharacterMovement`) "MOVE_None" 0)
  (`KismetSystemLibrary.Delay` 2.8)
  (`SceneComponent.SetVisibility` (`self.Widget`) false false)
  (`PrimitiveComponent.SetSimulatePhysics` (`self.Mesh`) true)
  (`PrimitiveComponent.SetSimulatePhysics` (`self.WeaponMesh`) true)
  (`CharacterMovementComponent.SetMovementMode` (`Character.CharacterMovement` (`GameplayStatics.GetPlayerCharacter` 0)) "MOVE_Walking" 0)
  (`|SpawnActorFromClass` "/Game/Consumables/Coin1.Coin1_C" (`SceneComponent.K2_GetComponentToWorld` (`self.DropLocation`)) "Undefined" "OverrideRootScale" null null)
  (`ActorComponent.K2_DestroyComponent` (`self.CapsuleComponent`))
  (`KismetSystemLibrary.Delay` 2.0)
  (`self.K2_DestroyActor`))

(event `ValueChecker`
  (if (<= (`self.Health`) 0.0)
    (`KismetSystemLibrary.Delay` 0.2)
    (`|SpawnActorFromClass` "/Game/Consumables/Coin.Coin_C" (`SceneComponent.K2_GetComponentToWorld` (`self.DropLocation`)) "Undefined" "OverrideRootScale" null null)
    (`SceneComponent.SetVisibility` (`self.Widget`) false false)
    (`PrimitiveComponent.SetSimulatePhysics` (`self.Mesh`) true)
    (`PrimitiveComponent.SetSimulatePhysics` (`self.WeaponMesh`) true)
    (`ActorComponent.K2_DestroyComponent` (`self.CapsuleComponent`))
    (`KismetSystemLibrary.Delay` 3.0)
    (`self.K2_DestroyActor`)))

(event `self.Sphere.OnComponentBeginOverlap`
  (params (OverlappedComponent :type "PrimitiveComponent Object Reference") (OtherActor :type "Actor Object Reference") (OtherComp :type "PrimitiveComponent Object Reference") (OtherBodyIndex :type Integer) (bFromSweep :type Boolean) (SweepResult :type "HitResult Structure (by ref)"))
  (cast `/Game/Blueprints/PlayerCharacter/PlayerCharacterBare_BP` OtherActor)
  (`SceneComponent.SetVisibility` (`self.Widget`) true false))

(event `self.Sphere.OnComponentEndOverlap`
  (params (OverlappedComponent :type "PrimitiveComponent Object Reference") (OtherActor :type "Actor Object Reference") (OtherComp :type "PrimitiveComponent Object Reference") (OtherBodyIndex :type Integer))
  (cast `/Game/Blueprints/PlayerCharacter/PlayerCharacterBare_BP` OtherActor)
  (`SceneComponent.SetVisibility` (`self.Widget`) false false))

(event `/Game/Blueprints/NPC/NPC2/AI/NPC_AI_INT.NPCMelee_Attack`
  (`|PlayMontage` (`self.Mesh`) "/Game/Characters/NPC/Animation/NPCSword_Combo_1_Montage.NPCSword_Combo_1_Montage"))

(event `self.ReceiveAnyDamage`
  (params (Damage :type "Float (single-precision)") (DamageType :type "DamageType Object Reference") (InstigatedBy :type "Controller Object Reference") (DamageCauser :type "Actor Object Reference"))
  ;[1 1 1] Take Damage and reset attack if hit
  (bind _output_get (set `self.Health` (- (`self.Health`) Damage)))
  (set `/Game/Blueprints/NPC/NPC2/AI/AI_HealthBarWB.Health` _output_get (`self.HealthWidgetREF`))
  (`self.PlayAnimMontage` "/Game/Characters/NPC2/Animation/Standing_React_Small_From_Left_Montage.Standing_React_Small_From_Left_Montage")
  (`self.ValueChecker`))

(event `self.SwordHitBox.OnComponentBeginOverlap`
  (params (OverlappedComponent :type "PrimitiveComponent Object Reference") (OtherActor :type "Actor Object Reference") (OtherComp :type "PrimitiveComponent Object Reference") (OtherBodyIndex :type Integer) (bFromSweep :type Boolean) (SweepResult :type "HitResult Structure (by ref)"))
  ;[1 1 1] Deal Damage
  (bind _asplayer_character_bare_bp (cast `/Game/Blueprints/PlayerCharacter/PlayerCharacterBare_BP` OtherActor))
  (if (`self.AttackReady_0`)
    (`/Engine/EditorBlueprintResources/StandardMacros.DoOnce` false :!label _label
      (:`Completed`
        (`GameplayStatics.ApplyDamage` _asplayer_character_bare_bp 10.0)
        (`KismetSystemLibrary.Delay` 0.4)
        (goto _label :!via `Reset`)))))

(fn `CanStealth`
  (returns (CanStealth :type Boolean))
  (return (`BlackboardComponent.GetValueAsBool` (`AIBlueprintHelperLibrary.GetBlackboard` (`self.GetController`)) "CanStealth")))

(fn `UserConstructionScript`)