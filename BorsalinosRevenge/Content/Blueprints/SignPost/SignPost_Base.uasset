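; Base signpost actor that shows its text on screen while the player character stands near it.
; A Box trigger creates a SignPost widget on overlap by PlayerCharacterBare_BP, adds it to the viewport and passes in the actor's Text.
; Leaving the box removes the widget and clears its reference.
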(event `self.Box.OnComponentBeginOverlap`
  (params (OverlappedComponent :type "PrimitiveComponent Object Reference") (OtherActor :type "Actor Object Reference") (OtherComp :type "PrimitiveComponent Object Reference") (OtherBodyIndex :type Integer) (bFromSweep :type Boolean) (SweepResult :type "HitResult Structure (by ref)"))
  (cast `/Game/Blueprints/PlayerCharacter/PlayerCharacterBare_BP` OtherActor)
  (bind _returnvalue (`|CreateWidget` "/Game/Blueprints/SignPost/SignPost_Widget.SignPost_Widget_C" (`GameplayStatics.GetPlayerController` 0)))
  (bind _output_get (set `self.SignPost_Widget` _returnvalue))
  (`UserWidget.AddToViewport` _output_get 0)
  (set `/Game/Blueprints/SignPost/SignPost_Widget.SignPostText` (`self.Text`) (`self.SignPost_Widget`)))

(event `self.Box.OnComponentEndOverlap`
  (params (OverlappedComponent :type "PrimitiveComponent Object Reference") (OtherActor :type "Actor Object Reference") (OtherComp :type "PrimitiveComponent Object Reference") (OtherBodyIndex :type Integer))
  (bind _signpost_widget (`self.SignPost_Widget`))
  (cast `/Game/Blueprints/PlayerCharacter/PlayerCharacterBare_BP` OtherActor)
  (`/Engine/EditorBlueprintResources/StandardMacros.IsValid` _signpost_widget
    (:`Is Valid`
      (`Widget.RemoveFromParent` _signpost_widget)
      (set `self.SignPost_Widget` null))))

(fn `UserConstructionScript`)