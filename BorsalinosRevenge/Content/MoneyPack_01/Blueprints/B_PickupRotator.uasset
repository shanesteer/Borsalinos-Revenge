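; Pickup actor that spins and bobs in place until an overlap collects it.
; Construction applies the configurable mesh, rotation offset and RotatingMovement rate.
; WiggleTimeline lerps the mesh between the root location and a WiggleLocation offset, alternating play and reverse to loop, with play rate set by inverse WiggleSpeed.
; Any actor overlap calls OnCollect, a placeholder that destroys the actor and prints an example "+1".
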(event `self.ReceiveBeginPlay`
  ;[1 1 1] Triggering Pickup Object Movement
  (`self.MoveUp`))

(event `MoveUp`
  ;[1 1 1] Pickup Object Wiggle Speed Control
  (`TimelineComponent.SetPlayRate` (`self.WiggleTimeline`) (/ 1.0 (`self.Wiggle Speed`)))
  ;[1 1 1] Pickup Object Movement Loop
  (bind (_direction _wiggle) (`Timeline|WiggleTimeline` :!via `PlayFromStart` :!label _label)
    (:`Update`
      (`self.Wiggle` _wiggle))
    (:`Finished`
      (switch `ETimelineDirection` _direction ; Timeline direction switch used to loop pickup movement
        (:`Forward`
          (`self.MoveDown`))
        (:`Backward`
          (`self.MoveUp`))))))

(event `MoveDown`
  ;[1 1 1] Pickup Object Wiggle Speed Control
  (`TimelineComponent.SetPlayRate` (`self.WiggleTimeline`) (/ 1.0 (`self.Wiggle Speed`)))
  (goto _label :!via `ReverseFromEnd`))

(event `self.ReceiveActorBeginOverlap`
  (params (OtherActor :type "Actor Object Reference"))
  ;[1 1 1] "On Collect" function call / Collecting Pickup Object
  (`self.OnCollect`))

(fn `OnCollect`
  ;[1 1 1] Your "OnCollect" code goes here. PrintString used as an example
  (`self.K2_DestroyActor`) ; Removes PickupObject from Level
  (`KismetSystemLibrary.PrintString` "+1") ; Example
)

(fn `UserConstructionScript`
  ;[1 1 1] Pick-up Object Rotation offset / Rotation rate setup
  (`SceneComponent.K2_SetRelativeRotation` (`self.PickupMesh`) (`self.Initial Rotation Offset`) false false)
  (set `RotatingMovementComponent.RotationRate` (`self.Rotation Rate`) (`self.RotatingMovement`))
  ;[1 1 1] Custom StaticMesh for Pickup Object
  (`StaticMeshComponent.SetStaticMesh` (`self.PickupMesh`) (`self.Mesh`)))

(fn `Wiggle`
  (params (Alpha :type "Float (double-precision)"))
  (bind _returnvalue (`SceneComponent.K2_GetComponentLocation` (`self.DefaultSceneRoot`)))
  ;[1 1 1] Pickup Object Location update
  (`SceneComponent.K2_SetWorldLocation` (`self.PickupMesh`) (`KismetMathLibrary.VLerp` _returnvalue (+ _returnvalue (`self.Wiggle Location`)) Alpha) false false))