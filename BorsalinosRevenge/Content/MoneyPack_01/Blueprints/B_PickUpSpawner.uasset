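; B_PickUpSpawner places rotating pickups evenly along a spline.
; SplineDivision divides the spline length by the Offset spacing to get the loop count.
; The construction script adds billboard components at those points as an editor preview.
; On BeginPlay it spawns B_PickupRotator actors at the same distances in world space, passing the mesh, rotation and wiggle speed settings.
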(event `self.ReceiveBeginPlay`
  ;[1 1 1] Loop Iterations based on Spline Chunks Calculation
  (for _index (range (+ (`self.SplineDivision`) 1))
    ;[1 1 1] Spawning Pickup Objects along the Spline (in Game)
    (`|SpawnActorFromClass` "/Game/MoneyPack_01/Blueprints/B_PickupRotator.B_PickupRotator_C" (`KismetMathLibrary.MakeTransform` (`SplineComponent.GetLocationAtDistanceAlongSpline` (`self.Spline`) (* _index (`self.Offset`)) "World")) "Undefined" "OverrideRootScale" null (`self.Initial Rotation Offset`) (`self.Rotation Rate`) (0.0 0.0 0.0) (`self.Wiggle Speed`) (`self.Mesh`))))

(fn `SplineDivision`
  (returns (NumberOfChunks :type Integer))
  ;[1 1 1] Even Spline Division based on Offset Variable
  (return (`KismetMathLibrary.FTrunc` (/ (`SplineComponent.GetSplineLength` (`self.Spline`)) (`self.Offset`)))))

(fn `UserConstructionScript`
  ;[1 1 1] Loop Iterations based on Spline Chunks Calculation
  (for _index (range (+ (`self.SplineDivision`) 1))
    ;[1 1 1] Spawning Preview Billboards along the Spline (Editor Preview)
    (`AddComponent|BillboardComponent_355` :`RelativeTransform` (`KismetMathLibrary.MakeTransform` (`SplineComponent.GetLocationAtDistanceAlongSpline` (`self.Spline`) (* _index (`self.Offset`)) "Local")))))